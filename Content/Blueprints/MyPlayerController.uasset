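; Player controller that switches between flying a pawn and editing a MySphere actor through a SphereEdit widget.
; In fly mode, gated axis inputs drive the pawn's floating movement and controller look.
; A Left Alt flip-flop alternates between line-tracing ahead for a sphere to load into the widget and enter edit mode, and hiding it to resume flight.
; Mouse cursor visibility doubles as the mode state.
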(event EventBeginPlay
  (CallFunction|InitPawn)
  (CallFunction|InitSphereWidget))

(event Input|AxisEvents|InputAxisMoveForward
  (params (AxisValue :type Float%20%28single-precision%29))
  (Utilities|IfinFlyMode
    (:IfInFlyMode
      (CallFunction|MoveForward AxisValue))))

(event Input|AxisEvents|InputAxisMoveRight
  (params (AxisValue :type Float%20%28single-precision%29))
  (Utilities|IfinFlyMode
    (:IfInFlyMode
      (CallFunction|MoveRight AxisValue))))

(event Input|AxisEvents|InputAxisLookUp
  (params (AxisValue :type Float%20%28single-precision%29))
  (Utilities|IfinFlyMode
    (:IfInFlyMode
      (CallFunction|LookUp AxisValue))))

(event Input|AxisEvents|InputAxisLookRight
  (params (AxisValue :type Float%20%28single-precision%29))
  (Utilities|IfinFlyMode
    (:IfInFlyMode
      (CallFunction|LookRight AxisValue))))

(event Input|AxisEvents|InputAxisMoveUpGlobal
  (params (AxisValue :type Float%20%28single-precision%29))
  (Utilities|IfinFlyMode
    (:IfInFlyMode
      (CallFunction|MoveUpGlobal AxisValue))))

(event Input|KeyboardEvents|LeftAlt
  (params (Key :type Key%20Structure))
  (bind _spherewidget (Variables|Default|GetSphereWidget))
  (:Pressed
    (Utilities|FlowControl|FlipFlop
      (:A
        (bind _sphere (Utilities|LookforSphereAhead)
          (:Found
            (Default|Readfrom _spherewidget _sphere)
            (Default|Show _spherewidget)
            (CallFunction|ToEditMode))))
      (:B
        (Default|Hide _spherewidget)
        (CallFunction|ToFlyMode)))))

(fn ConstructionScript)

(fn InitPawn
  (bind _asmy_pawn (Utilities|Casting|CastToMyPawn (Pawn|GetControlledPawn)))
  (Variables|Default|SetMyPawn _asmy_pawn))

(fn MoveForward
  (params (A :type Float%20%28single-precision%29))
  (bind _mypawn (Variables|Default|GetMyPawn))
  (Class|PawnMovementComponent|AddInputVector (Variables|/Game/Blueprints/MyPawn.MyPawn_C|GetFloatingPawnMovement _mypawn) (* (Math|Vector|GetForwardVector (Variables|/Game/Blueprints/MyPawn.MyPawn_C|GetSphere _mypawn)) (* A 5e+01)) false))

(fn MoveRight
  (params (A :type Float%20%28single-precision%29))
  (bind _mypawn (Variables|Default|GetMyPawn))
  (Class|PawnMovementComponent|AddInputVector (Variables|/Game/Blueprints/MyPawn.MyPawn_C|GetFloatingPawnMovement _mypawn) (* (Math|Vector|GetRightVector (Variables|/Game/Blueprints/MyPawn.MyPawn_C|GetSphere _mypawn)) (* A 5e+01)) false))

(fn LookUp
  (params (A :type Float%20%28single-precision%29))
  (Class|PlayerController|AddPitchInput A))

(fn LookRight
  (params (A :type Float%20%28single-precision%29))
  (Class|PlayerController|AddYawInput A))

(fn MoveUpGlobal
  (params (Axis :type Float%20%28single-precision%29))
  (Class|PawnMovementComponent|AddInputVector (Variables|/Game/Blueprints/MyPawn.MyPawn_C|GetFloatingPawnMovement (Variables|Default|GetMyPawn)) (* (Math|Vector|VectorUp) (* Axis 5e+01)) false))

(fn InitSphereWidget
  (bind _returnvalue (UserInterface|CreateWidget "/Game/Widgets/SphereEdit.SphereEdit_C" self))
  (bind _output_get (Variables|Default|SetSphereWidget _returnvalue))
  (Default|Hide _output_get)
  (UserInterface|Viewport|AddtoViewport _output_get 0))

(fn ToEditMode
  (Variables|Default|SetbShowMouseCursor true))

(fn ToFlyMode
  (Variables|Default|SetbShowMouseCursor false))

(fn IsinEditMode
  (return (Variables|Default|GetbShowMouseCursor)))

(fn IsinFlyMode
  (return (not (Variables|Default|GetbShowMouseCursor))))